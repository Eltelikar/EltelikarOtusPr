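; BP_InventoryItem is a world item actor that can be picked up into an inventory through an Interact event.
; Its construction script builds a BP_BaseItemObject from the actor's display, count and equipment type properties plus its own class, storing it as DefaultObjectReference.
; On interaction, it passes that object to the inventory's AddItemToInventory and destroys itself only if the add succeeds.
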(event `/Game/Inventory/BPI_Interact.Interact`
  (params (Inventory :type "/Game/Inventory/BPC_Inventory Object Reference"))
  (`self.InteractItem` Inventory))

(fn `InteractItem`
  (params (Inventory :type "/Game/Inventory/BPC_Inventory Object Reference"))
  (bind _add_ (`/Game/Inventory/BPC_Inventory.AddItemToInventory` Inventory (`self.DefaultObjectReference`)))
  (if _add_
    (`self.K2_DestroyActor`)))

(fn `UserConstructionScript`
  (bind _returnvalue (`|GenericCreateObject` "/Game/Inventory/BP_BaseItemObject.BP_BaseItemObject_C" (`self.Image`) (`GameplayStatics.GetObjectClass` self) (`self.Name`) (`self.Desctription`) (`self.Count`) (`self.Equipment Type`)))
  (set `self.DefaultObjectReference` _returnvalue))