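; Inventory component that stores items and equipment, toggles the grid inventory UI and handles interaction with world objects.
; BeginPlay fills the inventory and equipment arrays with placeholder item objects; adding replaces the first one lacking a valid ItemReference and refreshes any open widget.
; While enabled, Tick sphere-traces from the follow camera to set the current target, which Interact messages with this component.
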(event `self.ReceiveTick`
  (params (DeltaSeconds :type "Float (single-precision)"))
  (if (`self.ActiveTracerInteract?`)
    (`self.TraceInteract` 0.0)))

(event `self.ReceiveBeginPlay`
  (`self.InitializationInventory`)
  (`self.InitializationEquipmentSlot`))

(fn `AddItemToInventory`
  (params (ItemToAdd :type "/Game/Inventory/BP_BaseItemObject Object Reference (by ref)"))
  (returns (`Add?` :type Boolean))
  (locals (EmptySlotIndex :type Integer) (`FindEmptySlot?` :type Boolean))
  (bind _ui_inventory_reference (`self.UI_Inventory_Reference`))
  (for (_array_element _array_index) (`self.Inventory`)
    (`/Engine/EditorBlueprintResources/StandardMacros.IsValid` _array_element
      (:`Is Valid`
        (if (`KismetSystemLibrary.IsValidClass` (`/Game/Inventory/BP_BaseItemObject.ItemReference` _array_element))
          (set `local.FindEmptySlot?` false)
          (else
            (set `local.EmptySlotIndex` _array_index)
            (set `local.FindEmptySlot?` true)
            (break))))))
  (if (`local.FindEmptySlot?`)
    (`KismetArrayLibrary.Array_Set` (`self.Inventory`) (`local.EmptySlotIndex`) (`local.ItemToAdd`))
    (`/Engine/EditorBlueprintResources/StandardMacros.IsValid` _ui_inventory_reference
      (:`Is Valid`
        (`/Game/Inventory/Widget/UI_InventoryGrid.Refresh_Inventory` _ui_inventory_reference))
      (:`Is Not Valid`
        _))
    (return true)
    (else
      (`KismetSystemLibrary.PrintString` "Inventory is full")
      (return false))))

(fn `InitializationEquipmentSlot`
  (for _ (range 12)
    (`|GenericCreateObject` "/Game/Inventory/BP_BaseItemObject.BP_BaseItemObject_C" null null)
    (`KismetArrayLibrary.Array_AddUnique` (`self.EquipmentSlots`))))

(fn `InitializationInventory`
  (for _ (range (+ (`self.InventorySize`) 1))
    (bind _returnvalue (`|GenericCreateObject` "/Game/Inventory/BP_BaseItemObject.BP_BaseItemObject_C" null null))
    (`KismetArrayLibrary.Array_AddUnique` (`self.Inventory`) _returnvalue)))

(fn `Interact`
  (bind _current_interact_item (`self.Current Interact Item`)
    (:`then`
      (message `/Game/Inventory/BPI_Interact.Interact` _current_interact_item self))
    (:`else`)))

(fn `Toggle Inentory`
  (bind _returnvalue (`GameplayStatics.GetPlayerController` 0))
  (bind _returnvalue_2 (`GameplayStatics.GetPlayerController` 0))
  (bind _ui_inventory_reference (`self.UI_Inventory_Reference`)
    (:`then`
      (`Widget.RemoveFromParent` _ui_inventory_reference)
      (set `PlayerController.bShowMouseCursor` false _returnvalue)
      (`WidgetBlueprintLibrary.SetInputMode_GameOnly` _returnvalue)
      (set `self.UI_Inventory_Reference` null))
    (:`else`
      (bind _returnvalue_3 (`|CreateWidget` "/Game/Inventory/Widget/UI_InventoryGrid.UI_InventoryGrid_C"))
      (bind _output_get (set `self.UI_Inventory_Reference` _returnvalue_3))
      (`UserWidget.AddToViewport` _output_get 0)
      (set `PlayerController.bShowMouseCursor` true _returnvalue_2)
      (`WidgetBlueprintLibrary.SetInputMode_GameAndUIEx` _returnvalue_2 (`self.UI_Inventory_Reference`)))))

(fn `TraceInteract`
  (params (LenghtTrace :type "Float (double-precision)"))
  (bind _followcamera (`/Game/ThirdPerson/Blueprints/BP_ThirdPersonCharacter.FollowCamera` (`self.BP_ThirdPersonCharacter`)))
  (bind _returnvalue (`SceneComponent.K2_GetComponentLocation` _followcamera))
  (bind _outhit (`KismetSystemLibrary.SphereTraceSingle` _returnvalue (+ _returnvalue (* (`SceneComponent.GetForwardVector` _followcamera) (`self.LenghtTrace`))) 15.0 "TraceTypeQuery1" false (`|MakeArray` null :!type "Actor Object Reference")))
  (bind (_bblockinghit _binitialoverlap _time _distance _location _impactpoint _normal _impactnormal _physmat _hitactor) (`GameplayStatics.BreakHitResult` _outhit))
  (if _bblockinghit
    (set `self.Current Interact Item` _hitactor)
    (else
      (set `self.Current Interact Item` null))))