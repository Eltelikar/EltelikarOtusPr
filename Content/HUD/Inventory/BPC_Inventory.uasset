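; Inventory component that manages the player's items, equipment slots, inventory panel and item interaction.
; On BeginPlay it fills both arrays with placeholder item objects; adding an item replaces the first slot lacking an item class and refreshes the open grid.
; While enabled, Tick sphere-traces from the follow camera, at zero length, to pick the Interact target.
; Equipping spawns and socket-attaches actors by equipment type, unequipping destroys them, and EquipArmor is empty.
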(event `self.ReceiveTick`
  (params (DeltaSeconds :type "Float (single-precision)"))
  (if (`self.ActiveTracerInteract?`)
    (`self.Trace Interact` 0.0)
    (if false
      (`|ExecutionSequence`
        (:`then_0`
          (for _array_element (`self.EquipmentSlots`)
            (bind _name (`/Game/HUD/Inventory/BP_BaseItemObject.Name` _array_element))
            (`KismetSystemLibrary.PrintString` (select `bool` (== _name (`|FormatText` "")) :`false` (`KismetTextLibrary.Conv_TextToString` _name) :`true` "Empty") true true (struct :`G` 1.0 :`B` 0.586081 :`A` 1.0) 0.0)))
        (:`then_1`
          (for _array_element_2 (`self.Inventory`)
            (bind _name_2 (`/Game/HUD/Inventory/BP_BaseItemObject.Name` _array_element_2))
            (`KismetSystemLibrary.PrintString` (select `bool` (== _name_2 (`|FormatText` "")) :`false` (`KismetTextLibrary.Conv_TextToString` _name_2) :`true` "Empty") true true (struct :`R` 0.951201 :`G` 1.0 :`A` 1.0) 0.0)))))))

(event `self.ReceiveBeginPlay`
  (`self.InitializationInventory`)
  (`self.InitializationEquipmentSlot`))

(fn `AddItemToInventory`
  (params (ItemToAdd :type "/Game/HUD/Inventory/BP_BaseItemObject Object Reference (by ref)"))
  (returns (`Add?` :type Boolean))
  (locals (EmptySlotIndex :type Integer) (`FindEmptySlot?` :type Boolean))
  (bind _ui_inventory_reference (`self.UI_Inventory_Reference`))
  (for (_array_element _array_index) (`self.Inventory`)
    (`/Engine/EditorBlueprintResources/StandardMacros.IsValid` _array_element
      (:`Is Valid`
        (if (`KismetSystemLibrary.IsValidClass` (`/Game/HUD/Inventory/BP_BaseItemObject.ItemReference` _array_element))
          (set `local.FindEmptySlot?` false)
          (else
            (set `local.EmptySlotIndex` _array_index)
            (set `local.FindEmptySlot?` true)
            (break))))))
  (if (`local.FindEmptySlot?`)
    (`KismetArrayLibrary.Array_Set` (`self.Inventory`) (`local.EmptySlotIndex`) (`local.ItemToAdd`))
    (`/Engine/EditorBlueprintResources/StandardMacros.IsValid` _ui_inventory_reference
      (:`Is Valid`
        (`/Game/HUD/Inventory/Widget/UI_InventoryGrid.Refresh_Inventory2` (`/Game/HUD/Inventory/Widget/UI_PlayerInfoPanel.UI_InventoryGrid` _ui_inventory_reference)))
      (:`Is Not Valid`
        _))
    (return true)
    (else
      (`KismetSystemLibrary.PrintString` "Inventory is full")
      (return false))))

(fn `EquipArmor`)

(fn `EquipWeapon`
  (params (Item :type "/Game/HUD/Inventory/BP_BaseItemObject Object Reference"))
  (locals (L_SpawnWeaponToEquip :type "/Game/HUD/Inventory/BP_InventoryItem Object Reference"))
  (bind _equipment_type (`/Game/HUD/Inventory/BP_BaseItemObject.Equipment Type` Item))
  (bind _l_spawnweapontoequip (`local.L_SpawnWeaponToEquip`))
  (bind _returnvalue (`|SpawnActorFromClass` (`/Game/HUD/Inventory/BP_BaseItemObject.ItemReference` Item) (`KismetMathLibrary.MakeTransform` (0.0 0.0 0.0)) "Undefined" "MultiplyWithRoot" null "NewEnumerator10" "NewEnumerator0" null))
  (bind _output_get (set `local.L_SpawnWeaponToEquip` _returnvalue))
  (`Actor.K2_AttachToComponent` _output_get (`Character.Mesh` (`self.BP_ThirdPersonCharacter`)) (`BlueprintMapLibrary.Map_Find` (`self.EquipmentSockets`) _equipment_type) "SnapToTarget" "SnapToTarget" "KeepRelative" true)
  (switch `/Game/HUD/Inventory/E_EquipmentType` _equipment_type
    (:`NewEnumerator4`
      (set `self.OneHandEquipReference` _l_spawnweapontoequip))
    (:`NewEnumerator14`
      (set `self.TwoHandEquipReference` _l_spawnweapontoequip))
    (:`NewEnumerator5`
      (set `self.SecondEquipReference` _l_spawnweapontoequip))
    (:`NewEnumerator12`
      (set `self.BowEquipReference` _l_spawnweapontoequip))
    (:`NewEnumerator13`
      (set `self.ArrowsEquipReference` _l_spawnweapontoequip))
    (:`NewEnumerator7`
      (set `self.FirstConsumablesEquipReference` _l_spawnweapontoequip))
    (:`NewEnumerator8`
      (set `self.SecConsumablesEquipReference` _l_spawnweapontoequip))
    (:`NewEnumerator15`
      (set `self.FreeEquipReference` _l_spawnweapontoequip))))

(fn `InitializationEquipmentSlot`
  (for _ (range 12)
    (`|GenericCreateObject` "/Game/HUD/Inventory/BP_BaseItemObject.BP_BaseItemObject_C" "NewEnumerator10" null null)
    (`KismetArrayLibrary.Array_AddUnique` (`self.EquipmentSlots`))))

(fn `InitializationInventory`
  (for _ (range 1 (+ (`self.InventorySize`) 1))
    (bind _returnvalue (`|GenericCreateObject` "/Game/HUD/Inventory/BP_BaseItemObject.BP_BaseItemObject_C" "NewEnumerator10" null null))
    (`KismetArrayLibrary.Array_AddUnique` (`self.Inventory`) _returnvalue)))

(fn `Interact`
  (bind _current_interact_item (`self.Current Interact Item`)
    (:`then`
      (`|ExecutionSequence`
        (:`then_0`
          (message `InteractiveInterface.OnInteract` _current_interact_item null))
        (:`then_1`
          (message `/Game/HUD/Inventory/BPI_Interact.Interact` _current_interact_item self))))
    (:`else`)))

(fn `Toggle Inentory`
  (bind _returnvalue (`GameplayStatics.GetPlayerController` 0))
  (bind _returnvalue_2 (`GameplayStatics.GetPlayerController` 0))
  (bind _ui_inventory_reference (`self.UI_Inventory_Reference`)
    (:`then`
      (`Widget.RemoveFromParent` _ui_inventory_reference)
      (set `PlayerController.bShowMouseCursor` false _returnvalue)
      (`WidgetBlueprintLibrary.SetInputMode_GameOnly` _returnvalue)
      (set `self.UI_Inventory_Reference` null))
    (:`else`
      (bind _returnvalue_3 (`|CreateWidget` "/Game/HUD/Inventory/Widget/UI_PlayerInfoPanel.UI_PlayerInfoPanel_C"))
      (bind _output_get (set `self.UI_Inventory_Reference` _returnvalue_3))
      (`UserWidget.AddToViewport` _output_get 0)
      (set `PlayerController.bShowMouseCursor` true _returnvalue_2)
      (`WidgetBlueprintLibrary.SetInputMode_GameAndUIEx` _returnvalue_2 (`self.UI_Inventory_Reference`)))))

(fn `Trace Interact`
  (params (LenghtTrace :type "Float (double-precision)"))
  (bind _followcamera (`/Game/ThirdPerson/Blueprints/BP_ThirdPersonCharacter.FollowCamera` (`self.BP_ThirdPersonCharacter`)))
  (bind _returnvalue (`SceneComponent.K2_GetComponentLocation` _followcamera))
  (bind _asbp_third_person_character (cast `/Game/ThirdPerson/Blueprints/BP_ThirdPersonCharacter` (`GameplayStatics.GetPlayerCharacter` 0)))
  (set `self.BP_ThirdPersonCharacter` _asbp_third_person_character)
  (bind _outhit (`KismetSystemLibrary.SphereTraceSingle` _returnvalue (+ _returnvalue (* (`SceneComponent.GetForwardVector` _followcamera) (`self.LenghtTrace`))) 15.0 "TraceTypeQuery3" false (`|MakeArray` null :!type "Actor Object Reference") "ForOneFrame" true (struct :`G` 0.936956 :`B` 1.0 :`A` 1.0) (struct :`G` 1.0 :`A` 1.0) 0.0))
  (bind (_bblockinghit _binitialoverlap _time _distance _location _impactpoint _normal _impactnormal _physmat _hitactor) (`GameplayStatics.BreakHitResult` _outhit))
  (if _bblockinghit
    (bind _output_get (set `self.Current Interact Item` _hitactor))
    (`KismetSystemLibrary.PrintString` (`KismetSystemLibrary.GetDisplayName` _output_get) true true (struct :`G` 1.0 :`B` 0.116071 :`A` 1.0) 0.0)
    (else
      (bind _output_get_2 (set `self.Current Interact Item` null))
      (`KismetSystemLibrary.PrintString` (`KismetSystemLibrary.GetDisplayName` _output_get_2) true true (struct :`R` 1.0 :`G` 0.028711 :`A` 1.0) 0.0))))

(fn `UnEquipWeapon`
  (params (ItemToUnEquip :type "/Game/HUD/Inventory/BP_BaseItemObject Object Reference"))
  (bind _arrowsequipreference (`self.ArrowsEquipReference`))
  (bind _secconsumablesequipreference (`self.SecConsumablesEquipReference`))
  (switch `/Game/HUD/Inventory/E_EquipmentType` (`/Game/HUD/Inventory/BP_BaseItemObject.Equipment Type` ItemToUnEquip)
    (:`NewEnumerator4`
      (`Actor.K2_DestroyActor` (`self.OneHandEquipReference`)))
    (:`NewEnumerator14`
      (`Actor.K2_DestroyActor` (`self.TwoHandEquipReference`)))
    (:`NewEnumerator5`
      (`Actor.K2_DestroyActor` (`self.SecondEquipReference`)))
    (:`NewEnumerator12`
      (`Actor.K2_DestroyActor` (`self.BowEquipReference`)))
    (:`NewEnumerator13`
      (set `/Game/HUD/Inventory/BP_BaseItemObject.Count` (`/Game/HUD/Inventory/BP_InventoryItem.Count` _arrowsequipreference) (`local.ItemToUnEquip`))
      (`Actor.K2_DestroyActor` _arrowsequipreference))
    (:`NewEnumerator7`
      (set `/Game/HUD/Inventory/BP_BaseItemObject.Count` 0 (`local.ItemToUnEquip`))
      (`Actor.K2_DestroyActor` (`self.FirstConsumablesEquipReference`)))
    (:`NewEnumerator8`
      (set `/Game/HUD/Inventory/BP_BaseItemObject.Count` (`/Game/HUD/Inventory/BP_InventoryItem.Count` _secconsumablesequipreference) (`local.ItemToUnEquip`))
      (`Actor.K2_DestroyActor` _secconsumablesequipreference))))